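; Boots slow pickup that alters the velocity of the ThirdPersonCharacter that overlaps it.
; On overlap it sets movement Velocity to a low X-only vector once and hides its mesh.
; After a ten-second delay it sets player 0's Velocity to a faster X vector and destroys itself.
; It writes Velocity directly rather than a max speed, and its JumpZVelocity nodes are unconnected.
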(event EventBeginPlay)

(event Collision|EventActorBeginOverlap
  (params (OtherActor :type Actor%20Object%20Reference))
  (bind _asthird_person_character (Utilities|Casting|CastToThirdPersonCharacter OtherActor))
  (Variables|/Script/Engine.MovementComponent|SetVelocity (Variables|/Script/Engine.Character|GetCharacterMovement _asthird_person_character) "20.000000, 0, 0")
  (Rendering|SetVisibility (Variables|Default|GetStaticMesh) false false)
  (Utilities|FlowControl|Delay 1e+01)
  (bind _asthird_person_character_2 (Utilities|Casting|CastToThirdPersonCharacter (Game|GetPlayerCharacter 0)))
  (Variables|/Script/Engine.MovementComponent|SetVelocity (Variables|/Script/Engine.Character|GetCharacterMovement _asthird_person_character_2) "600.000000, 0, 0")
  (Actor|DestroyActor))

(event EventTick
  (params (DeltaSeconds :type Float%20%28single-precision%29)))

(fn ConstructionScript)