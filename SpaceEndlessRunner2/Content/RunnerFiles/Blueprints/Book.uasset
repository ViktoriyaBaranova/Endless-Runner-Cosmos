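; Book pickup actor that rewards the player with coins and opens a book screen when touched.
; On overlap with ThirdPersonCharacter, it adds a fixed amount to the Coins counter on ThirdPersonGameMode and hides its mesh.
; It then pauses the game, adds a ForBookBP widget to the viewport and destroys itself after a player-character cast whose result is unused.
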(event EventBeginPlay)

(event Collision|EventActorBeginOverlap
  (params (OtherActor :type Actor%20Object%20Reference))
  (Utilities|Casting|CastToThirdPersonCharacter OtherActor)
  (bind _asthird_person_game_mode (Utilities|Casting|CastToThirdPersonGameMode (Game|GetGameMode)))
  (Variables|/Game/ThirdPersonBP/Blueprints/ThirdPersonGameMode.ThirdPersonGameMode_C|SetCoins _asthird_person_game_mode (+ (Variables|/Game/ThirdPersonBP/Blueprints/ThirdPersonGameMode.ThirdPersonGameMode_C|GetCoins _asthird_person_game_mode) 50))
  (Rendering|SetVisibility (Variables|Default|GetStaticMesh) false false)
  (Game|SetGamePaused true)
  (bind _returnvalue (UserInterface|CreateWidget "/Game/RunnerFiles/UI/BookBP/ForBookBP.ForBookBP_C"))
  (UserInterface|Viewport|AddtoViewport _returnvalue 0)
  (Utilities|Casting|CastToThirdPersonCharacter (Game|GetPlayerCharacter 0))
  (Actor|DestroyActor))

(event EventTick
  (params (DeltaSeconds :type Float%20%28single-precision%29)))

(fn ConstructionScript)